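; Player pawn that possesses itself on BeginPlay and drives a physics Cube with WASD and the mouse.
; Key events set movement flags, and Tick applies a velocity-change impulse each frame for every active flag, unscaled by delta time.
; Forward follows the Cube's forward vector, while back, left and right push along fixed world axes.
; Mouse X yaws the Cube and Mouse Y pitches the SpringArm, inverted from the axis value.
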(event `self.ReceiveBeginPlay`
  (`Controller.Possess` (`GameplayStatics.GetPlayerController` 0) self))

(event `Key|W`
  (params (Key :type "Key Structure"))
  (:`Pressed`
    (set `self.MoveForward?` true))
  (:`Released`
    (set `self.MoveForward?` false)))

(event `Key|A`
  (params (Key :type "Key Structure"))
  (:`Pressed`
    (set `self.MoveLeft?` true))
  (:`Released`
    (set `self.MoveLeft?` false)))

(event `self.ReceiveTick`
  (params (DeltaSeconds :type "Float (single-precision)"))
  (bind _cube (`self.Cube`))
  (bind _cube_2 (`self.Cube`))
  (`|ExecutionSequence`
    (:`then_0`
      (if (`self.MoveForward?`)
        (`PrimitiveComponent.AddImpulse` _cube (* (`SceneComponent.GetForwardVector` _cube) 50.0) "None" true)))
    (:`then_1`
      (if (`self.MoveBacl?`)
        (`PrimitiveComponent.AddImpulse` _cube_2 (-50.0 0.0 0.0) "None" true)))
    (:`then_2`
      (if (`self.MoveLeft?`)
        (`PrimitiveComponent.AddImpulse` _cube_2 (0.0 -50.0 0.0) "None" true)))
    (:`then_3`
      (if (`self.MoveRight?`)
        (`PrimitiveComponent.AddImpulse` _cube_2 (0.0 50.0 0.0) "None" true)))))

(event `Key|D`
  (params (Key :type "Key Structure"))
  (:`Pressed`
    (set `self.MoveRight?` true))
  (:`Released`
    (set `self.MoveRight?` false)))

(event `Key|S`
  (params (Key :type "Key Structure"))
  (:`Pressed`
    (set `self.MoveBacl?` true))
  (:`Released`
    (set `self.MoveBacl?` false)))

(event `InputAxisKey|MouseX`
  (params (AxisValue :type "Float (single-precision)"))
  (`SceneComponent.K2_AddRelativeRotation` (`self.Cube`) (`KismetMathLibrary.MakeRotator` 0.0 0.0 AxisValue) false false))

(event `InputAxisKey|MouseY`
  (params (AxisValue :type "Float (single-precision)"))
  (`SceneComponent.K2_AddRelativeRotation` (`self.SpringArm`) (`KismetMathLibrary.MakeRotator` 0.0 (* AxisValue -1.0)) false false))

(fn `UserConstructionScript`)